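; WinZone is a JackBall level's goal volume that also runs level UI, music, death and pause handling.
; BeginPlay shows the level-number HUD and starts BGM, which fades on any overlap as the win sound plays.
; For JackBall_Character, overlap saves the next unlock (capped at MaxLevel) and best score to LevelInfo, then shows the win widget paused.
; DeathEvent stops music and shows the death widget paused after a delay; Pause forwards to the HUD.
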(event OnComponentBeginOverlap(CollisionComponent)
  (params (OverlappedComponent :type Primitive%20Component%20Object%20Reference) (OtherActor :type Actor%20Object%20Reference) (OtherComp :type Primitive%20Component%20Object%20Reference) (OtherBodyIndex :type Integer) (bFromSweep :type Boolean) (SweepResult :type Hit%20Result%20Structure%20%28by%20ref%29))
  (bind _levelnumber (Variables|Default|GetLevelNumber))
  (bind _returnvalue (- _levelnumber 1))
  (bind _returnvalue_2 (+ _levelnumber 1))
  (Audio|Components|Audio|FadeOut (Variables|Default|GetSound2D) 1.0 0.1 :!class /Script/Engine.AudioComponent)
  (Audio|PlaySound2D "/Game/JackBall/Sounds/Win2.Win2")
  (bind _asjack_ball_character (Utilities|Casting|CastToJackBall_Character OtherActor))
  (bind _returnvalue_3 (SaveGame|LoadGamefromSlot "LevelInfo"))
  (bind _aslevel_info (Utilities|Casting|CastToLevelInfo _returnvalue_3))
  (if (and (< (Variables|/Game/JackBall/Blueprints/LevelInfo.LevelInfo_C|GetLevelUntil _aslevel_info) _returnvalue_2) (<= _returnvalue_2 (Variables|/Game/JackBall/Blueprints/JackBallGameInstance.JackBallGameInstance_C|GetMaxLevel (.AsJack%20Ball%20Game%20Instance (Utilities|Casting|CastToJackBallGameInstance (Game|GetGameInstance))))))
    (Variables|/Game/JackBall/Blueprints/LevelInfo.LevelInfo_C|SetLevelUntil _aslevel_info _returnvalue_2))
  (if (< (Utilities|Array|Get(acopy) (Variables|/Game/JackBall/Blueprints/LevelInfo.LevelInfo_C|GetLevelScore _aslevel_info) _returnvalue) (Variables|/Script/JackBall.JackBall_Character|GetScore _asjack_ball_character))
    (Utilities|Array|SetArrayElem (Variables|/Game/JackBall/Blueprints/LevelInfo.LevelInfo_C|GetLevelScore _aslevel_info) _returnvalue (Variables|/Script/JackBall.JackBall_Character|GetScore _asjack_ball_character)))
  (SaveGame|SaveGametoSlot _aslevel_info "LevelInfo")
  (bind _returnvalue_4 (UserInterface|CreateWidget "/Game/JackBall/Blueprints/WidgetForWin.WidgetForWin_C"))
  (Variables|/Game/JackBall/Blueprints/WidgetForWin.WidgetForWin_C|SetNextLevel _returnvalue_4 (+ (Variables|Default|GetLevelNumber) 1))
  (UserInterface|Viewport|AddtoViewport _returnvalue_4 0)
  (Input|SetInputModeUIOnly (Game|GetPlayerController 0) _returnvalue_4 "DoNotLock")
  (Game|SetGamePaused true))

(event Custom|Pause
  (bind _foundwidgets (Widget|GetAllWidgetsOfClass "/Game/JackBall/Blueprints/UserInterface.UserInterface_C" true))
  (Default|Pause (Utilities|Array|Get(acopy) _foundwidgets)))

(event Custom|DeathEvent
  (Audio|Components|Audio|Stop (Variables|Default|GetSound2D))
  (Utilities|FlowControl|Delay 3.0)
  (Utilities|FlowControl|DoOnce false
    (:Completed
      (bind _returnvalue (UserInterface|CreateWidget "/Game/JackBall/Blueprints/WidgetForDead.WidgetForDead_C"))
      (UserInterface|Viewport|AddtoViewport _returnvalue 0)
      (Game|SetGamePaused true))))

(event EventBeginPlay
  (bind _returnvalue (UserInterface|CreateWidget "/Game/JackBall/Blueprints/UserInterface.UserInterface_C"))
  (Rendering|Components|TextRender|SetText (Variables|/Game/JackBall/Blueprints/UserInterface.UserInterface_C|GetTextBlock_0 _returnvalue) (Utilities|Text|FormatText "第{XX}关" (Variables|Default|GetLevelNumber)))
  (UserInterface|Viewport|AddtoViewport _returnvalue 0)
  (bind _returnvalue_2 (Audio|SpawnSound2D (Variables|Default|GetBGMToPlay)))
  (Variables|Default|SetSound2D _returnvalue_2))

(fn ConstructionScript)