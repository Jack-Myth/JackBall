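; JackBall game mode that sets up the mouse cursor and floor surface when play begins.
; BeginPlay shows the cursor, then reads the AllowSurfaceMaterial flag from the first actor tagged WinZone.
; When that flag is set, it loads the LevelInfo save slot and applies its saved FloorSurface material to every Floor_Blueprint actor in the level.
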(event EventBeginPlay
  (Variables|/Script/Engine.PlayerController|SetbShowMouseCursor (Game|GetPlayerController 0) true)
  (bind _outactors (Actor|GetAllActorswithTag "WinZone"))
  (bind _aswin_zone (Utilities|Casting|CastToWinZone (Utilities|Array|Get(acopy) _outactors)))
  (if (Variables|/Game/JackBall/Blueprints/WinZone.WinZone_C|GetAllowSurfaceMaterial _aswin_zone)
    (bind _returnvalue (SaveGame|LoadGamefromSlot "LevelInfo"))
    (bind _aslevel_info (Utilities|Casting|CastToLevelInfo _returnvalue))
    (bind _outactors_2 (Actor|GetAllActorsOfClass "/Game/JackBall/Blueprints/Floor_Blueprint.Floor_Blueprint_C"))
    (for _array_element _outactors_2
      (Rendering|Material|SetMaterial (Variables|/Script/Engine.StaticMeshActor|GetStaticMeshComponent _array_element) 0 (Variables|/Game/JackBall/Blueprints/LevelInfo.LevelInfo_C|GetFloorSurface _aslevel_info)))))

(fn ConstructionScript)